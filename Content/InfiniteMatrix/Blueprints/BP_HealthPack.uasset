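; BP_HealthPack is a health pickup that responds to BP_Player entering its HPTriggerZone.
; On overlap it asks HPSpawner to spawn HP at a spawn point and destroys itself; no healing is applied in this Blueprint.
; RandomizeHP sets WallHP to a random circle, pentagon, square or triangle mesh but is not called here.
; WallHP rotation logic exists but is disconnected and never runs.
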(event `self.ReceiveTick`
  (params (DeltaSeconds :type "Float (single-precision)")))

(event `self.HPTriggerZone.OnComponentBeginOverlap`
  (params (OverlappedComponent :type "PrimitiveComponent Object Reference") (OtherActor :type "Actor Object Reference") (OtherComp :type "PrimitiveComponent Object Reference") (OtherBodyIndex :type Integer) (bFromSweep :type Boolean) (SweepResult :type "HitResult Structure (by ref)"))
  (cast `/Game/InfiniteMatrix/Blueprints/BP_Player` OtherActor)
  (`/Game/InfiniteMatrix/Blueprints/BP_HPSpawner.SpawnHPAtSpawnPoint` (`self.HPSpawner`))
  (`self.K2_DestroyActor`))

(fn `RandomizeHP`
  (`StaticMeshComponent.SetStaticMesh` (`self.WallHP`) (select `int` (`KismetMathLibrary.RandomIntegerInRange` 0 3) :`0` "/Game/InfiniteMatrix/Meshes/SM_Circle.SM_Circle" :`1` "/Game/InfiniteMatrix/Meshes/SM_Pentagon.SM_Pentagon" :`2` "/Game/InfiniteMatrix/Meshes/SM_Square.SM_Square" :`3` "/Game/InfiniteMatrix/Meshes/SM_Triangle.SM_Triangle" :!type "StaticMesh Object Reference")))

(fn `UserConstructionScript`)