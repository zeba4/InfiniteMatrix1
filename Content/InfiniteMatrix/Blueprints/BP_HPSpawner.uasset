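; BP_HPSpawner is a spawner actor meant to lay a chain of BP_HealthPack pickups when play begins.
; SpawnInitialHP loops a few times, targeting the player pawn's location when no valid NewestHP exists, otherwise that pack's SpawnHPPoint.
; SpawnHP's body is disconnected from its entry, so nothing currently spawns.
; That unwired logic would spawn a pack, store it as NewestHP, give it a spawner reference and call RandomizeHP.
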(event `self.ReceiveBeginPlay`
  (`self.SpawnInitialHP`))

(fn `SpawnHP`
  (params (SpawnHPLocation :type "Vector Structure")))

(fn `SpawnHPAtSpawnPoint`
  (`self.SpawnHP` (`SceneComponent.K2_GetComponentLocation` (`/Game/InfiniteMatrix/Blueprints/BP_HealthPack.SpawnHPPoint` (`self.NewestHP`)))))

(fn `SpawnInitialHP`
  (for _ (range 3)
    (`/Engine/EditorBlueprintResources/StandardMacros.IsValid` (`self.NewestHP`)
      (:`Is Valid`
        (`self.SpawnHPAtSpawnPoint`))
      (:`Is Not Valid`
        (`self.SpawnHP` (`self.K2_GetActorLocation` (`GameplayStatics.GetPlayerPawn` 0)))))))

(fn `UserConstructionScript`)